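; Player controller for a Pokémon-style game that handles menu cursor visibility, Pokémon selection and healing items.
; Menu selection stores the chosen Pokémon and its image, then calls a battle-selection event that only prints debug text.
; Item use finds name matches in the array from menu selection and writes health plus heal value, unclamped, into BP_PlayerCharacter's health array at that character's selected index.
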(event `self.ReceiveBeginPlay`)

(event `self.ReceiveTick`
  (params (DeltaSeconds :type "Float (single-precision)")))

(event `/Game/Blueprints/Interfaces/BI_menuMouse.MenuAddPlayerMouse`
  ;[1 1 1] Adds Mouse To Screen
  (`self.AddMouse`))

(event `/Game/Blueprints/Interfaces/BI_menuMouse.MenuRemovePlayerMouse`
  ;[1 1 1] Removes Mouse from Screen
  (`self.RemoveMouse`))

(event `/Game/Blueprints/Interfaces/BI_SelectedPokemon.SelectCurrentPokemonMenu`
  (params (inputPokemon :type "/Game/Blueprints/Pokemon/Struct_PokemonTable Structure") (inputPokemonArray :type "Array of /Game/Blueprints/Pokemon/Struct_PokemonTable Structure (by ref)") (inputIndex :type Integer))
  ;[1 1 1] SELECT POINTING TO THE LAST
  (`self.CurrentSelectedPokemon` inputPokemon)
  (`/Game/Blueprints/Interfaces/BI_SelectedPokemon.SelectCurrentPokemonBattle` inputPokemon)
  (set `self.PokemonImageSlate` (`.PokemonImage_8_DD48773A4875BF1453FFCB8ED868C5FD` (break `/Game/Blueprints/Pokemon/Struct_PokemonTable` inputPokemon))))

(event `/Game/Blueprints/Interfaces/BI_ApplyObjectsOnToPokemon.ApplyitemsOnToPokemon`
  (params (itemInput :type "/Game/Blueprints/GameObjects/Items/Struc_ItemStructure Structure") (Health :type "Array of Float (single-precision) (by ref)"))
  ;[0.1996 1 0.3151] Heals pokemon from Items!
  (`self.Heal Pokemon` itemInput (stale `/Game/Blueprints/Interfaces/BI_SelectedPokemon.SelectCurrentPokemonMenu` inputPokemonArray) Health))

(event `/Game/Blueprints/Interfaces/BI_SelectedPokemon.SelectCurrentPokemonBattle`
  (params (inputPokemon :type "/Game/Blueprints/Pokemon/Struct_PokemonTable Structure"))
  (`KismetSystemLibrary.PrintString` "THIS LITERALLY TAKES THE DATA AND UPDATE IT FOR THE CURRENT BATTLE")
  (`KismetSystemLibrary.PrintString` (`KismetStringLibrary.Concat_StrStr` ":: POKEMON IS :::: " (`.PokemonName_2_C98A6A6D44977FF56A865D9F907BCF85` (break `/Game/Blueprints/Pokemon/Struct_PokemonTable` inputPokemon)))))

(fn `AddMouse`
  (set `self.bShowMouseCursor` true)
  (`KismetSystemLibrary.PrintString` "Add Mouse"))

(fn `CurrentSelectedPokemon`
  (params (NewParam :type "/Game/Blueprints/Pokemon/Struct_PokemonTable Structure"))
  ;[1 1 1] Literally selects the current pokemon
  (set `self.SelectedPokemon` NewParam))

(fn `Heal Pokemon`
  (params (inputItem :type "/Game/Blueprints/GameObjects/Items/Struc_ItemStructure Structure") (inputPokemonUpdate :type "Array of /Game/Blueprints/Pokemon/Struct_PokemonTable Structure") (inputPokemonHealth :type "Array of Float (double-precision)"))
  (bind _asbp_player_character (cast `/Game/Blueprints/Player/BP_PlayerCharacter` (`GameplayStatics.GetPlayerCharacter` 0)))
  (for _array_element inputPokemonUpdate
    (bind _pokemonname (break `/Game/Blueprints/Pokemon/Struct_PokemonTable` _array_element))
    (if (`KismetStringLibrary.EqualEqual_StrStr` _pokemonname (`.PokemonName_2_C98A6A6D44977FF56A865D9F907BCF85` (break `/Game/Blueprints/Pokemon/Struct_PokemonTable` (`self.SelectedPokemon`))))
      (bind _currentselectedpokemonindex (`/Game/Blueprints/Player/BP_PlayerCharacter.currentSelectedPokemonIndex` _asbp_player_character))
      (`KismetSystemLibrary.PrintString` (`KismetStringLibrary.Concat_StrStr` "POKEMON IS :::: " _pokemonname "REF    :::: " (`KismetStringLibrary.Conv_IntToString` _currentselectedpokemonindex)))
      (bind _output (`|GetArrayItem` inputPokemonHealth _currentselectedpokemonindex))
      (bind _returnvalue (+ _output (`.itemHealValue_20_210A93DC431C9EFF4922B4B92D6E5C8A` (break `/Game/Blueprints/GameObjects/Items/Struc_ItemStructure` inputItem))))
      (`KismetSystemLibrary.PrintString` (`KismetStringLibrary.Concat_StrStr` "HEALTH IN ::::" (`KismetStringLibrary.Conv_DoubleToString` _output) "ADD TO GET TOTAL OF :::: " (`KismetStringLibrary.Conv_DoubleToString` _returnvalue)))
      (`KismetArrayLibrary.Array_Set` (`/Game/Blueprints/Player/BP_PlayerCharacter.PokemonHealthAmount` _asbp_player_character) _currentselectedpokemonindex _returnvalue))))

(fn `RemoveMouse`
  (set `self.bShowMouseCursor` false)
  (`KismetSystemLibrary.PrintString` "Remove Mouse"))

(fn `UserConstructionScript`)