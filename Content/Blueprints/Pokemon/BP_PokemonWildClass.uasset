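; Wild Pokémon actor that shows a random species sprite and can serve as a starter choice.
; On BeginPlay it picks a random DT_PokemonType row within its number range and, if a starter, registers with the player character.
; A starter's first player overlap adds that row to the player's inventory immediately and opens the choose-Pokémon widget.
; Non-starters ignore overlaps, and DestroyPokemon lets other code remove the actor.
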(event `self.Box.OnComponentEndOverlap`
  (params (OverlappedComponent :type "PrimitiveComponent Object Reference") (OtherActor :type "Actor Object Reference") (OtherComp :type "PrimitiveComponent Object Reference") (OtherBodyIndex :type Integer))
  (cast `/Game/Blueprints/Player/BP_PlayerCharacter` OtherActor))

(event `self.Box.OnComponentBeginOverlap`
  (params (OverlappedComponent :type "PrimitiveComponent Object Reference") (OtherActor :type "Actor Object Reference") (OtherComp :type "PrimitiveComponent Object Reference") (OtherBodyIndex :type Integer) (bFromSweep :type Boolean) (SweepResult :type "HitResult Structure (by ref)"))
  (bind _asbp_player_character (cast `/Game/Blueprints/Player/BP_PlayerCharacter` OtherActor))
  (if (`self.StartingPokemon?`)
    (`/Engine/EditorBlueprintResources/StandardMacros.DoOnce` false
      (:`Completed`
        (message `/Game/Blueprints/Interfaces/BI_menuMouse.MenuAddPlayerMouse` (`GameplayStatics.GetPlayerController` 0))
        (bind _returnvalue (`|CreateWidget` "/Game/Blueprints/UMG/Player/HUD_ChooseThisPokemon.HUD_ChooseThisPokemon_C" null _asbp_player_character))
        (`KismetArrayLibrary.Array_Add` (`/Game/Blueprints/Player/BP_PlayerCharacter.InventoryPokemon` _asbp_player_character) (stale `self.ReceiveBeginPlay` _out_row))
        (set `/Game/Blueprints/UMG/Player/HUD_ChooseThisPokemon.SelectedPokemonName` (stale `self.ReceiveBeginPlay` _pokemonname) _returnvalue)
        (`UserWidget.AddToViewport` _returnvalue 0)))))

(event `self.ReceiveBeginPlay`
  (bind (_pokemonname _out_row) (`self.SetPokemon`))
  (bind _asbp_player_character (cast `/Game/Blueprints/Player/BP_PlayerCharacter` (`GameplayStatics.GetPlayerCharacter` 0)))
  (if (`self.StartingPokemon?`)
    (`KismetArrayLibrary.Array_Add` (`/Game/Blueprints/Player/BP_PlayerCharacter.PokemonStartStore` _asbp_player_character) self)))

(fn `DestroyPokemon`
  (`self.K2_DestroyActor`))

(fn `SetPokemon`
  (returns (PokemonName :type String) (`Out Row` :type "/Game/Blueprints/Pokemon/Struct_PokemonTable Structure"))
  (bind _returnvalue (`|GetDataTableRow` "/Game/Blueprints/Pokemon/DT_PokemonType.DT_PokemonType" (`KismetStringLibrary.Conv_StringToName` (`KismetStringLibrary.Conv_IntToString` (`KismetMathLibrary.RandomIntegerInRange` (`self.RoadNumberMinRange`) (`self.RoadNumberMaxRange`)))))
    (:`then`
      (bind (_pokemonname _pokemontype _pokemonimage) (break `/Game/Blueprints/Pokemon/Struct_PokemonTable` _returnvalue))
      (`PaperSpriteComponent.SetSprite` (`self.PaperSprite`) _pokemonimage)
      (return _pokemonname _returnvalue))))

(fn `UserConstructionScript`)