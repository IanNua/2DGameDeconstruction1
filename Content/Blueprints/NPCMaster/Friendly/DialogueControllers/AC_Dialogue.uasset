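; AC_Dialogue is an NPC dialogue component that runs branching conversations through an AI behavior tree.
; On BeginPlay it spawns its own AIC_Dialogue controller.
; InteractionConvo shows a HUD_Dialogue widget in UI-only input mode, runs the DialogueTree, and writes the widget and QuestPhaseID to the BB_Dialogue blackboard.
; The widget's OnExit event restores game input, stops the tree logic and removes the widget.
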(event `self.ReceiveBeginPlay`
  ;[1 1 1] SETS initial node controllers
  (bind _returnvalue (`|SpawnActorFromClass` "/Game/Blueprints/NPCMaster/Friendly/DialogueControllers/AIC_Dialogue.AIC_Dialogue_C" (`KismetMathLibrary.MakeTransform` (0.0 0.0 0.0)) "Undefined" "OverrideRootScale" null null))
  (set `self.AIC` _returnvalue))

(event `/Game/Blueprints/NPCMaster/Friendly/DialogueControllers/BI_Conversation.InteractionConvo`
  (params (playerRef :type "/Game/Blueprints/Player/BP_PlayerCharacter Object Reference"))
  (bind _aic (`self.AIC`))
  (bind _asbp_player_controller (cast `/Game/Blueprints/Player/BP_PlayerController` (`Pawn.GetController` playerRef) :!pure true))
  ;[1 1 1] Builds Dialogue Tree Based on Player interaction with NPC
  (`KismetSystemLibrary.PrintString` "CHECK POINT")
  (bind _returnvalue (`|CreateWidget` "/Game/Blueprints/UMG/Conversation/HUD_Dialogue.HUD_Dialogue_C" _asbp_player_controller (`self.NPCName`)))
  (bind _output_get (set `self.DialogueWidget` _returnvalue))
  (add `/Game/Blueprints/UMG/Conversation/HUD_Dialogue.onExit` _output_get (delegate `ExitEvent`))
  (`UserWidget.AddToViewport` _output_get 0)
  (`WidgetBlueprintLibrary.SetInputMode_UIOnlyEx` _asbp_player_controller _output_get)
  (set `PlayerController.bShowMouseCursor` true _asbp_player_controller)
  (`AIController.RunBehaviorTree` _aic (`self.DialogueTree`))
  (bind _blackboardcomponent (`AIController.UseBlackboard` _aic "/Game/Blueprints/NPCMaster/Friendly/DialogueControllers/BB_Dialogue.BB_Dialogue"))
  (`BlackboardComponent.SetValueAsObject` _blackboardcomponent "DialogueWidget" (`self.DialogueWidget`))
  (`BlackboardComponent.SetValueAsInt` _blackboardcomponent "QuestPhaseID" (`self.QuestPhaseID`)))

(event `ExitEvent`
  (bind _dialoguewidget (`self.DialogueWidget`))
  (bind _asbp_player_controller (cast `/Game/Blueprints/Player/BP_PlayerController` (`Widget.GetOwningPlayer` _dialoguewidget) :!pure true))
  ;[1 1 1] Ends Current Event for the Dialogue tree
  (`WidgetBlueprintLibrary.SetInputMode_GameOnly` _asbp_player_controller)
  (set `PlayerController.bShowMouseCursor` false _asbp_player_controller)
  (`BrainComponent.StopLogic` (`AIController.BrainComponent` (`self.AIC`)) "")
  (`Widget.RemoveFromParent` _dialoguewidget))