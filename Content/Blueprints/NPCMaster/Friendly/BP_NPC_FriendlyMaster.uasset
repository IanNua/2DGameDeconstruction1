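; Master Blueprint for friendly Paper2D NPCs that passes name and dialogue tree to its dialogue component.
; On overlapping PlayerFacingCollision, the player's look-at yaw picks a facing and matching flipbook by NPCIndex, with left and right sharing one flipbook via rotation.
; The player entering BattleZone briefly shows a text render.
; BuildPokemonRange is an empty stub, and the direction check leaves debug traces and prints active.
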(event `self.ReceiveBeginPlay`
  (bind _ac_dialogue (`self.AC_Dialogue`))
  (`self.BuildPokemonRange`)
  (`PaperFlipbookComponent.SetFlipbook` (`self.PaperFlipbook`) (`|GetArrayItem` (`.NpcDown_6_185C83C14F40D0D0E8E0CF991A0A3E81` (break `/Game/Blueprints/NPCMaster/SpriteBooks` (`self.npcFlipbook`))) (`self.NPCIndex`)))
  (set `/Game/Blueprints/NPCMaster/Friendly/DialogueControllers/AC_Dialogue.NPCName` (`self.NPCName`) _ac_dialogue)
  (set `/Game/Blueprints/NPCMaster/Friendly/DialogueControllers/AC_Dialogue.DialogueTree` (`self.Dialogue Tree`) _ac_dialogue))

(event `self.playerFacingCollision.OnComponentBeginOverlap`
  (params (OverlappedComponent :type "PrimitiveComponent Object Reference") (OtherActor :type "Actor Object Reference") (OtherComp :type "PrimitiveComponent Object Reference") (OtherBodyIndex :type Integer) (bFromSweep :type Boolean) (SweepResult :type "HitResult Structure (by ref)"))
  (bind _asbp_player_character (cast `/Game/Blueprints/Player/BP_PlayerCharacter` OtherActor))
  (`self.DeterminePlayerDirection` _asbp_player_character)
  (`self.SetFlipBook`))

(event `self.battleZone.OnComponentBeginOverlap`
  (params (OverlappedComponent :type "PrimitiveComponent Object Reference") (OtherActor :type "Actor Object Reference") (OtherComp :type "PrimitiveComponent Object Reference") (OtherBodyIndex :type Integer) (bFromSweep :type Boolean) (SweepResult :type "HitResult Structure (by ref)"))
  (cast `/Game/Blueprints/Player/BP_PlayerCharacter` OtherActor)
  (`SceneComponent.SetVisibility` (`self.TextRender`) true true)
  (`KismetSystemLibrary.Delay` 1.0)
  (`SceneComponent.SetVisibility` (`self.TextRender`) false false))

(event `self.battleZone.OnComponentEndOverlap`
  (params (OverlappedComponent :type "PrimitiveComponent Object Reference") (OtherActor :type "Actor Object Reference") (OtherComp :type "PrimitiveComponent Object Reference") (OtherBodyIndex :type Integer))
  (cast `/Game/Blueprints/Player/BP_PlayerCharacter` OtherActor)
  (`SceneComponent.SetVisibility` (`self.TextRender`) false false))

(fn `BuildPokemonRange`
  ;[1 1 1] Hold on this till later
)

(fn `DeterminePlayerDirection`
  (params (Target :type "Actor Object Reference"))
  (returns (EndPoint :type "Vector Structure"))
  (bind _returnvalue (`SceneComponent.K2_GetComponentLocation` (`self.PaperFlipbook`)))
  (bind _outhit (`KismetSystemLibrary.LineTraceSingle` :`Start` _returnvalue :`End` (`self.K2_GetActorLocation` Target) :`TraceChannel` "TraceTypeQuery1" :`DrawDebugType` "Persistent" :`TraceColor` (struct :`R` 1.0 :`B` 0.794383 :`A` 1.0) :`TraceHitColor` (struct :`R` 1.0 :`B` 0.007519 :`A` 1.0)))
  (bind (_bblockinghit _binitialoverlap _time _distance _location _impactpoint _normal _impactnormal _physmat _hitactor _hitcomponent _hitbonename _hititem _elementindex _faceindex _tracestart _traceend) (`GameplayStatics.BreakHitResult` _outhit))
  (bind _returnvalue_2 (`KismetMathLibrary.FindLookAtRotation` _returnvalue _traceend))
  (`KismetSystemLibrary.PrintString` (`KismetStringLibrary.Concat_StrStr` "DIRECT X Y Z :::: " (`KismetStringLibrary.Conv_RotatorToString` _returnvalue_2)))
  (bind _yaw (.yaw _returnvalue_2))
  (if (and (> _yaw -45.0) (< _yaw 45.0))
    (set `self.NPC Direction` "NewEnumerator0")
    (return _traceend)
    (elif (and (>= _yaw 45.0) (<= _yaw 135.0))
      (set `self.NPC Direction` "NewEnumerator2")
      (return _traceend)
      (elif (and (>= _yaw -135.0) (<= _yaw -45.0))
        (set `self.NPC Direction` "NewEnumerator3")
        (return _traceend)
        (else
          (set `self.NPC Direction` "NewEnumerator1")
          (return _traceend))))))

(fn `SetFlipBook`
  (bind _paperflipbook (`self.PaperFlipbook`))
  (bind _npcindex (`self.NPCIndex`))
  (bind (_npcdown _npcup _npcleft) (break `/Game/Blueprints/NPCMaster/SpriteBooks` (`self.npcFlipbook`)))
  (switch `/Game/Blueprints/NPCMaster/Enum_NPC_Direction` (`self.NPC Direction`)
    (:`NewEnumerator0`
      (`PaperFlipbookComponent.SetFlipbook` _paperflipbook (`|GetArrayItem` _npcup _npcindex)))
    (:`NewEnumerator1`
      (`PaperFlipbookComponent.SetFlipbook` _paperflipbook (`|GetArrayItem` _npcdown _npcindex)))
    (:`NewEnumerator2`
      (`SceneComponent.K2_SetRelativeRotation` _paperflipbook (struct :`Yaw` -90.0 :`Roll` 90.0) false false)
      (`PaperFlipbookComponent.SetFlipbook` _paperflipbook (`|GetArrayItem` _npcleft _npcindex)))
    (:`NewEnumerator3`
      (`SceneComponent.K2_SetRelativeRotation` _paperflipbook (struct :`Yaw` 90.0 :`Roll` -90.0) false false)
      (`PaperFlipbookComponent.SetFlipbook` _paperflipbook (`|GetArrayItem` _npcleft _npcindex)))))

(fn `UserConstructionScript`)